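; Cluster sub-bomb actor for the Clusterflack indirect weapon that detonates on a timer.
; Tick and the Update event both add world delta seconds to Timer.
; Once Timer passes TimeToExplode, it calls Explote, defined outside this graph, and spawns an ExplotionBP actor at its location with default rotation and scale.
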(event `self.ReceiveTick`
  (params (DeltaSeconds :type "Float (single-precision)"))
  (bind _output_get (set `self.timer` (+ (`GameplayStatics.GetWorldDeltaSeconds`) (`self.timer`)) :!label _label))
  (if (> _output_get (`self.timeToExplode`))
    (`self.explote`)
    (`|SpawnActorFromClass` "/Game/explotionBP.explotionBP_C" (`KismetMathLibrary.MakeTransform` (`self.K2_GetActorLocation`)) "Undefined" "OverrideRootScale" null null)))

(event `self.Update`
  (goto _label))

(fn `UserConstructionScript`)