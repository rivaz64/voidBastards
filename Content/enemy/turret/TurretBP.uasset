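; Enemy turret that pops up when the player character enters its detection sphere and retracts when they leave.
; Activate, allowed only while Damagable has Vida left, shows eye, gun and middle and raises the top; Deactivate reverses this, both setting an Activated flag.
; Died swaps the turret meshes for the destroyed one and removes the Live widget, an enemy life display bound to the turret on BeginPlay.
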(event `self.ReceiveBeginPlay`
  (bind _asenemy_var_life (cast `/Game/enemy/enemyVarLife` (`WidgetComponent.GetWidget` (`self.live`))))
  (set `/Game/enemy/enemyVarLife.actor` self _asenemy_var_life))

(event `self.activate`
  (if (> (`damagable.vida` (`self.damagable`)) 0)
    (`SceneComponent.SetVisibility` (`self.eye`) true false)
    (`SceneComponent.SetVisibility` (`self.gun`) true false)
    (`SceneComponent.SetVisibility` (`self.Middle`) true false)
    (`SceneComponent.K2_SetRelativeLocation` (`self.up`) (0.0 0.0 230.0) false false)
    (set `self.activated` true)))

(event `self.deactivate`
  (`SceneComponent.SetVisibility` (`self.eye`) false false)
  (`SceneComponent.SetVisibility` (`self.gun`) false false)
  (`SceneComponent.SetVisibility` (`self.Middle`) false false)
  (`SceneComponent.K2_SetRelativeLocation` (`self.up`) (0.0 0.0 160.0) false false)
  (set `self.activated` false))

(event `self.died`
  (bind _live (`self.live`))
  (`SceneComponent.SetVisibility` (`self.eye`) false false)
  (`SceneComponent.SetVisibility` (`self.gun`) false false)
  (`SceneComponent.SetVisibility` (`self.Destoyed`) true false)
  (`SceneComponent.SetVisibility` (`self.base`) false false)
  (`SceneComponent.SetVisibility` (`self.up`) false false)
  (`SceneComponent.SetVisibility` (`self.Middle`) false false)
  (`/Engine/EditorBlueprintResources/StandardMacros.IsValid` _live
    (:`Is Valid`
      (`ActorComponent.K2_DestroyComponent` _live))))

(event `self.Sphere.OnComponentBeginOverlap`
  (params (OverlappedComponent :type "PrimitiveComponent Object Reference") (OtherActor :type "Actor Object Reference") (OtherComp :type "PrimitiveComponent Object Reference") (OtherBodyIndex :type Integer) (bFromSweep :type Boolean) (SweepResult :type "HitResult Structure (by ref)"))
  (cast `voidBastardsCharacter` OtherActor)
  (`self.activate`))

(event `self.Sphere.OnComponentEndOverlap`
  (params (OverlappedComponent :type "PrimitiveComponent Object Reference") (OtherActor :type "Actor Object Reference") (OtherComp :type "PrimitiveComponent Object Reference") (OtherBodyIndex :type Integer))
  (cast `voidBastardsCharacter` OtherActor)
  (`self.deactivate`))

(fn `UserConstructionScript`)