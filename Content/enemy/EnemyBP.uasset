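; Enemy Blueprint with a Paper2D sprite, a life widget and a poison effect.
; BeginPlay links the widget to the actor and sets the idle group; Tick applies the current Anims sprite, mirroring it through negative X scale, and offsets SphereF along velocity.
; Pawn sensing and FeelNear overlaps both call OnSeen.
; Events swap normal and hit materials, set sprite yaw and activate poison; Died only prints a debug string.
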(event `self.ReceiveBeginPlay`
  (bind _asenemy_var_life (cast `/Game/enemy/enemyVarLife` (`WidgetComponent.GetWidget` (`self.life`))))
  (set `/Game/enemy/enemyVarLife.actor` self _asenemy_var_life)
  (set `self.actualGroup` (`self.idleF`)))

(event `self.setNormalMaterial`
  (`PrimitiveComponent.SetMaterial` (`self.PaperSprite`) 0 (`self.MaterialNormal`)))

(event `self.setHittedMaterial`
  (`PrimitiveComponent.SetMaterial` (`self.PaperSprite`) 0 (`self.MaterialHitted`)))

(event `self.setSpriteRotation`
  (params (angle :type "Float (single-precision)"))
  (`SceneComponent.K2_SetWorldRotation` (`self.PaperSprite`) (`KismetMathLibrary.MakeRotator` 0.0 0.0 angle) false false))

(event `self.ReceiveTick`
  (params (DeltaSeconds :type "Float (single-precision)"))
  (bind (_x _y) (`KismetMathLibrary.BreakVector2D` (* (`KismetMathLibrary.NormalSafe2D` (`KismetMathLibrary.MakeVector2D` (.x (`self.GetVelocity`)) (.y (`self.GetVelocity`))) 0.01) (100.0 100.0))))
  (`|ExecutionSequence`
    (:`then_0`
      (bind _aspaper_sprite (cast `PaperSprite` (`Animation.sprite` (`self.anims`))))
      (`PaperSpriteComponent.SetSprite` (`self.PaperSprite`) _aspaper_sprite)
      (if (`Animation.inverted` (`self.anims`))
        (`self.invertSprite`)
        (else
          (`self.normalSprite`))))
    (:`then_1`
      (`SceneComponent.K2_SetRelativeLocation` (`self.SphereF`) (`KismetMathLibrary.MakeVector` _x _y) false false))))

(event `self.normalSprite`
  (bind _papersprite (`self.PaperSprite`))
  (`SceneComponent.SetWorldScale3D` _papersprite (`KismetMathLibrary.MakeVector` (`KismetMathLibrary.Abs` (.x (`SceneComponent.K2_GetComponentScale` _papersprite))) (.y (`SceneComponent.K2_GetComponentScale` _papersprite)) (.z (`SceneComponent.K2_GetComponentScale` _papersprite))))
  (`SceneComponent.K2_SetRelativeRotation` (`self.life`) (struct :`Yaw` 90.0) false false))

(event `self.invertSprite`
  (bind _papersprite (`self.PaperSprite`))
  (`SceneComponent.SetWorldScale3D` _papersprite (`KismetMathLibrary.MakeVector` (- 0.0 (`KismetMathLibrary.Abs` (.x (`SceneComponent.K2_GetComponentScale` _papersprite)))) (.y (`SceneComponent.K2_GetComponentScale` _papersprite)) (.z (`SceneComponent.K2_GetComponentScale` _papersprite))))
  (`SceneComponent.K2_SetRelativeRotation` (`self.life`) (struct :`Yaw` 90.0 :`Roll` 180.0) false false))

(event `self.onPoised`
  (`ActorComponent.Activate` (`self.poisoned`) false))

(event `self.died`
  (`KismetSystemLibrary.PrintString` "Hello"))

(event `self.PawnSensing.OnSeePawn`
  (params (Pawn :type "Pawn Object Reference"))
  (`self.onSeen`))

(event `self.feelNear.OnComponentBeginOverlap`
  (params (OverlappedComponent :type "PrimitiveComponent Object Reference") (OtherActor :type "Actor Object Reference") (OtherComp :type "PrimitiveComponent Object Reference") (OtherBodyIndex :type Integer) (bFromSweep :type Boolean) (SweepResult :type "HitResult Structure (by ref)"))
  (`self.onSeen`))

(fn `UserConstructionScript`)