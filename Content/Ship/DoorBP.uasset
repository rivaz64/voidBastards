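; Ship door Blueprint that slides vertically open while pawns stand in its trigger box and it is unlocked, and closes otherwise.
; Box overlap events count pawns inside, and Tick moves the Door component up or down at Vel within a fixed height range.
; The change event toggles the lock and swaps the HandPanel material between green and red to show the state.
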(event `self.ReceiveTick`
  (params (DeltaSeconds :type "Float (single-precision)"))
  (bind _door (`self.door`))
  (bind _door_2 (`self.door`))
  (if (`self.unlocked`)
    (if (== (`self.inside`) 0)
      (if (> (.z (`SceneComponent.RelativeLocation` _door_2)) 0.0) :!label _label
        (`SceneComponent.K2_AddRelativeLocation` _door_2 (`KismetMathLibrary.MakeVector` 0.0 0.0 (* DeltaSeconds -1.0 (`self.vel`))) false false))
      (elif (< (.z (`SceneComponent.RelativeLocation` _door)) 250.0)
        (`SceneComponent.K2_AddRelativeLocation` _door (`KismetMathLibrary.MakeVector` 0.0 0.0 (* DeltaSeconds (`self.vel`))) false false)))
    (else
      (goto _label))))

(event `self.Box.OnComponentBeginOverlap`
  (params (OverlappedComponent :type "PrimitiveComponent Object Reference") (OtherActor :type "Actor Object Reference") (OtherComp :type "PrimitiveComponent Object Reference") (OtherBodyIndex :type Integer) (bFromSweep :type Boolean) (SweepResult :type "HitResult Structure (by ref)"))
  (cast `Pawn` OtherActor)
  (`/Engine/EditorBlueprintResources/StandardMacros.IncrementInt` (`self.inside`)))

(event `self.Box.OnComponentEndOverlap`
  (params (OverlappedComponent :type "PrimitiveComponent Object Reference") (OtherActor :type "Actor Object Reference") (OtherComp :type "PrimitiveComponent Object Reference") (OtherBodyIndex :type Integer))
  (cast `Pawn` OtherActor)
  (`/Engine/EditorBlueprintResources/StandardMacros.DecrementInt` (`self.inside`)))

(event `change`
  (bind _handpanel (`self.HandPanel`))
  (bind _output_get (set `self.unlocked` (not (`self.unlocked`))))
  (if _output_get
    (`PrimitiveComponent.SetMaterial` _handpanel 0 (`self.matGren`))
    (else
      (`PrimitiveComponent.SetMaterial` _handpanel 0 (`self.matRed`)))))

(fn `UserConstructionScript`)